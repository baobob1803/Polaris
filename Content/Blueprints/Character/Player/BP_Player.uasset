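; Player Blueprint that manages a scrollable weapon inventory, a held shield and basic health.
; Picked-up weapons are stored once in an array and attached to WeaponSlot; scrolling wraps through the array, toggling visibility to swap the equipped one.
; Shield input shows or hides the shield component.
; Health starts at the ACStats maximum via Saving, which persists nothing; Dead only prints, and the primary weapon action is unwired.
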(event Custom|PickUpWeapon
  (params (WeaponToPickUp :type BP%20C%20Weapons%20Object%20Reference))
  (if (not (Utilities|Array|ContainsItem (Variables|WeaponManagement|GetListOfOwnedWeapons) WeaponToPickUp))
    (Utilities|Array|Add (Variables|WeaponManagement|GetListOfOwnedWeapons) WeaponToPickUp)
    (Variables|WeaponManagement|SetWeaponToEquip WeaponToPickUp)
    (for _array_element (Variables|WeaponManagement|GetListOfOwnedWeapons)
      (Development|PrintString (Utilities|GetObjectName _array_element)))
    (CallFunction|InitializeWeapon WeaponToPickUp)))

(event Custom|InitializeWeapon
  (params (WeaponToRetrieve :type BP%20C%20Weapons%20Object%20Reference))
  (Transformation|AttachComponentToComponent WeaponToRetrieve (Variables|Default|GetWeaponSlot) "None" "SnapToTarget" "KeepRelative" "KeepWorld" true)
  (CallFunction|UpdateWeapon))

(event Custom|SwitchWeapon
  (bind _listofownedweapons (Variables|WeaponManagement|GetListOfOwnedWeapons))
  (bind _currentequipedweapon (Variables|WeaponManagement|GetCurrentEquipedWeapon))
  (bind _scrolling (Variables|WeaponManagement|GetScrolling))
  (bind _returnvalue (Utilities|Array|FindItem _listofownedweapons _currentequipedweapon))
  (bind _returnvalue_2 (+ _returnvalue _scrolling))
  (if (== _returnvalue_2 (Utilities|Array|Length (Variables|WeaponManagement|GetListOfOwnedWeapons)))
    (Variables|WeaponManagement|SetWeaponToEquipIndex 0)
    (elif (< _returnvalue_2 0)
      (Variables|WeaponManagement|SetWeaponToEquipIndex (- (Utilities|Array|Length (Variables|WeaponManagement|GetListOfOwnedWeapons)) 1))
      (else
        (Variables|WeaponManagement|SetWeaponToEquipIndex _returnvalue_2))))
  (bind _output_get (Variables|WeaponManagement|SetWeaponToEquip (Utilities|Array|Get(acopy) (Variables|WeaponManagement|GetListOfOwnedWeapons) (Variables|WeaponManagement|GetWeaponToEquipIndex))))
  (Development|PrintString (Utilities|GetObjectName _output_get) true true "(R=1.000000,G=0.000000,B=0.053850,A=1.000000)")
  (CallFunction|UpdateWeapon))

(event Custom|UpdateWeapon
  (bind _weapontoequip (Variables|WeaponManagement|GetWeaponToEquip))
  (bind _listofownedweapons (Variables|WeaponManagement|GetListOfOwnedWeapons))
  (bind _returnvalue (Utilities|Array|FindItem _listofownedweapons _weapontoequip))
  (bind _output (Utilities|Array|Get(acopy) _listofownedweapons _returnvalue))
  (if (Utilities|IsValid (Variables|WeaponManagement|GetCurrentEquipedWeapon))
    (Rendering|SetVisibility (Variables|/Script/Engine.Actor|GetRootComponent (Variables|WeaponManagement|GetCurrentEquipedWeapon)) false true)
    (Collision|SetCollisionEnabled (Variables|/Game/Blueprints/World/Weapons/BP_CWeapons.BP_CWeapons_C|GetSphere (Variables|WeaponManagement|GetCurrentEquipedWeapon)) "NoCollision"))
  (Rendering|SetVisibility (Variables|/Script/Engine.Actor|GetRootComponent _output) true true)
  (Collision|SetCollisionEnabled (Variables|/Game/Blueprints/World/Weapons/BP_CWeapons.BP_CWeapons_C|GetSphere _output) "NoCollision")
  (Variables|WeaponManagement|SetCurrentEquipedWeapon (Variables|WeaponManagement|GetWeaponToEquip)))

(event EventBeginPlay
  (CallFunction|Saving))

(event Input|ActionEvents|InputActionScrollWeaponUp
  (params (Key :type Key%20Structure :default "None"))
  (:Pressed
    (Variables|WeaponManagement|SetScrolling 1)
    (CallFunction|SwitchWeapon)))

(event Input|ActionEvents|InputActionScrollWeaponDown
  (params (Key :type Key%20Structure :default "None"))
  (:Pressed
    (Variables|WeaponManagement|SetScrolling -1)
    (CallFunction|SwitchWeapon)))

(event Input|ActionEvents|InputActionLMB
  (params (Key :type Key%20Structure :default "None")))

(event Input|ActionEvents|InputActionShield
  (params (Key :type Key%20Structure :default "None"))
  (:Pressed
    (Development|PrintString "Shield Up")
    (Development|SetHiddeninGame (Variables|Default|GetShield) false false))
  (:Released
    (Development|PrintString "Shield Down")
    (Development|SetHiddeninGame (Variables|Default|GetShield) true false)))

(fn ConstructionScript)

(fn Saving
  (Variables|Default|SetCurrentHealth (Utilities|Struct|BreakST_Stats (Variables|/Game/Blueprints/AC/AC_Stats.AC_Stats_C|GetStats (Variables|Default|GetAC_Stats))))
  (Development|PrintString "SAVED" true true "(R=0.000000,G=1.000000,B=0.110465,A=1.000000)"))

(fn CheckLife
  (if (<= (Variables|Default|GetCurrentHealth) 0)
    (Variables|Default|SetIsDead true)
    (else
      (Variables|Default|SetIsDead false)))
  (return (Variables|Default|GetIsDead)))

(fn TakeDamage
  (params (Damage%20to%20inflict :type Integer))
  (Variables|Default|SetCurrentHealth (- (Variables|Default|GetCurrentHealth) Damage%20to%20inflict)))

(fn Dead
  (Development|PrintString "Dead"))