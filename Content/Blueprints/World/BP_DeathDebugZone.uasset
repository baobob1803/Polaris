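; BP_DeathDebugZone is a debug damage volume that hurts or kills BP_Player on overlap, printing health or death messages.
; BeginPlay caches the player and sets the sphere's material according to InstantKill.
; With InstantKill, overlap deals max-health damage; otherwise a delayed loop applies DamageInflicted until the player leaves or CheckLife returns true.
; Death is handed to the player's Dead function.
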(event OnComponentBeginOverlap(Sphere1)
  (params (OverlappedComponent :type Primitive%20Component%20Object%20Reference) (OtherActor :type Actor%20Object%20Reference) (OtherComp :type Primitive%20Component%20Object%20Reference) (OtherBodyIndex :type Integer) (bFromSweep :type Boolean) (SweepResult :type Hit%20Result%20Structure%20%28by%20ref%29))
  (bind _playerref (Variables|Default|GetPlayerRef))
  (if (== OtherActor (Variables|Default|GetPlayerRef))
    (Variables|Default|SetPlayerIsIn true)
    (if (Variables|Default|GetInstantKill)
      (Default|TakeDamage _playerref (Utilities|Struct|BreakST_Stats (Variables|/Game/Blueprints/AC/AC_Stats.AC_Stats_C|GetStats (Variables|/Game/Blueprints/Character/Player/BP_Player.BP_Player_C|GetAC_Stats _playerref))))
      (bind _isplayerdead (Default|CheckLife _playerref))
      (if _isplayerdead
        (Default|Dead _playerref)
        (Development|PrintString "DEADDDDD"))
      (else
        (while (Variables|Default|GetPlayerIsIn)
          (Utilities|FlowControl|Delay (Variables|Default|GetDamageLoop))
          (Default|TakeDamage (Variables|Default|GetPlayerRef) (Variables|Default|GetDamageInflicted))
          (Development|PrintString (Utilities|String|ToString(Integer) (Variables|/Game/Blueprints/Character/Player/BP_Player.BP_Player_C|GetCurrentHealth (Variables|Default|GetPlayerRef))) true true "(R=1.000000,G=0.774734,B=0.000000,A=1.000000)")
          (bind _isplayerdead_2 (Default|CheckLife (Variables|Default|GetPlayerRef)))
          (if _isplayerdead_2
            (Variables|Default|SetPlayerIsIn false)))
        (if (Variables|/Game/Blueprints/Character/Player/BP_Player.BP_Player_C|GetIsDead (Variables|Default|GetPlayerRef))
          (Default|Dead (Variables|Default|GetPlayerRef)))
        (Development|PrintString (Utilities|String|ToString(Text) (Utilities|Text|FormatText "Current Health is {playerHealth}" (Variables|/Game/Blueprints/Character/Player/BP_Player.BP_Player_C|GetCurrentHealth (Variables|Default|GetPlayerRef)))) true true "(R=0.586574,G=1.000000,B=0.000000,A=1.000000)")))))

(event OnComponentEndOverlap(Sphere1)
  (params (OverlappedComponent :type Primitive%20Component%20Object%20Reference) (OtherActor :type Actor%20Object%20Reference) (OtherComp :type Primitive%20Component%20Object%20Reference) (OtherBodyIndex :type Integer))
  (if (== OtherActor (Variables|Default|GetPlayerRef))
    (Variables|Default|SetPlayerIsIn false)))

(event EventBeginPlay
  (bind _returnvalue (Actor|GetActorOfClass "/Game/Blueprints/Character/Player/BP_Player.BP_Player_C"))
  (Variables|Default|SetPlayerRef _returnvalue)
  (if (Variables|Default|GetInstantKill)
    (Rendering|Material|SetMaterial (Variables|Default|GetSphere) 0 "/Game/FPWeapon/Materials/FirstPersonProjectileMaterial.FirstPersonProjectileMaterial")
    (else
      (Rendering|Material|SetMaterial (Variables|Default|GetSphere) 0 "/Game/FPWeapon/Materials/BaseMaterial.BaseMaterial"))))

(fn ConstructionScript)