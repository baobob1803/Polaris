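; BP_RailGun is a rail gun weapon that the player picks up by walking into it.
; When its Sphere overlaps an actor whose class is exactly BP_Player, it passes itself to that player's PickUpWeapon and disables the sphere's collision.
; BeginPlay and the construction script only call the parent, and UsePrimaryAction is an empty stub, so no firing behavior is defined here.
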(event OnComponentBeginOverlap(Sphere)
  (params (OverlappedComponent :type Primitive%20Component%20Object%20Reference) (OtherActor :type Actor%20Object%20Reference) (OtherComp :type Primitive%20Component%20Object%20Reference) (OtherBodyIndex :type Integer) (bFromSweep :type Boolean) (SweepResult :type Hit%20Result%20Structure%20%28by%20ref%29))
  (if (== (Utilities|GetClass OtherActor) "/Game/Blueprints/Character/Player/BP_Player.BP_Player_C")
    (bind _asbp_player (Utilities|Casting|CastToBP_Player OtherActor))
    (Default|PickUpWeapon _asbp_player self)
    (Collision|SetCollisionEnabled (Variables|Default|GetSphere) "NoCollision")))

(event EventBeginPlay
  (|CallParentFunction))

(fn ConstructionScript
  (|CallParentFunction))

(fn UsePrimaryAction)